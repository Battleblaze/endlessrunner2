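; Game mode for an endless runner that creates the UI and persists high scores.
; On BeginPlay it creates the WDG_UI widget, hands it a game mode reference and adds it to the screen.
; SaveGameEvent appends the current HighScore to the array in the loaded BP_Save and sorts it, or creates a new save if none exists.
; Either path writes back to the slot with an async save.
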(event `self.ReceiveBeginPlay`
  (bind _asbp_myendlessrunner_2game_mode_base (cast `/Game/BPs/BP_Myendlessrunner2GameModeBase` (`GameplayStatics.GetGameMode`)))
  (bind _returnvalue (`|CreateWidget` "/Game/BPs/WDG_UI.WDG_UI_C"))
  (set `/Game/BPs/WDG_UI.GameModeRef` _asbp_myendlessrunner_2game_mode_base _returnvalue)
  (`UserWidget.AddToPlayerScreen` _returnvalue 0))

(event `self.SaveGameEvent`
  (bind _returnvalue (`GameplayStatics.LoadGameFromSlot` (`self.SlotString`)))
  (if (`KismetSystemLibrary.IsValid` _returnvalue)
    (bind _asbp_save (cast `/Game/BPs/BP_Save` _returnvalue))
    (bind _highscorearray (`/Game/BPs/BP_Save.HighScoreArray` _asbp_save))
    (`KismetArrayLibrary.Array_Add` _highscorearray (`self.highScore`))
    (bind _returnvalue_2 (`self.SortArray` _highscorearray))
    (set `/Game/BPs/BP_Save.HighScoreArray` _returnvalue_2 _asbp_save)
    (`AsyncActionHandleSaveGame.AsyncSaveGameToSlot` _asbp_save (`self.SlotString`))
    (else
      (bind _returnvalue_3 (`GameplayStatics.CreateSaveGameObject` "/Game/BPs/BP_Save.BP_Save_C"))
      (set `/Game/BPs/BP_Save.HighScoreArray` (`|MakeArray` (`self.highScore`) :!type "Float (double-precision)") _returnvalue_3)
      (`AsyncActionHandleSaveGame.AsyncSaveGameToSlot` _returnvalue_3 (`self.SlotString`)
        (:`Completed`
          (`KismetSystemLibrary.PrintString` "Created new save file"))))))

(fn `UserConstructionScript`)